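; BP_BrickPileAuto is a building-art prop that procedurally lays out a row of brick instances.
; The construction script adds Num instances to the Tile component, spaced by Interval along Dir with random jitter masked by RandomPannerMask.
; Alternate instances get a Panner offset and RotationPanner rotation, and InvertSort flips which parity receives them.
; Scale applies to all instances except the offset ones in inverted mode.
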(event EventBeginPlay)

(event Collision|EventActorBeginOverlap
  (params (OtherActor :type Actor%20Object%20Reference)))

(event EventTick
  (params (DeltaSeconds :type Float%20%28single-precision%29)))

(fn ConstructionScript
  (bind _randomrange (Variables|Default|GetRandomRange))
  (bind _rotationpanner (Variables|Default|GetRotationPanner))
  (bind _scale (Variables|Default|Getscale))
  (for _index (range 0 (- (Variables|Default|GetNum) 1))
    (if (Variables|Default|GetInvertSort)
      (if (== (Math|Integer|%(Integer) _index 2) 0)
        (Components|InstancedStaticMesh|AddInstance (Variables|Default|GetTile) (Math|Transform|MakeTransform (+ (* _index (* (Variables|Default|GetDir) (Variables|Default|GetInterval))) (* (Math|Random|RandomFloatinRange (* -1.0 _randomrange) _randomrange) (Variables|Default|GetRandomPannerMask))) "0, 0, 0" _scale) false)
        (else
          (Components|InstancedStaticMesh|AddInstance (Variables|Default|GetTile) (Math|Transform|MakeTransform (+ (+ (* _index (* (Variables|Default|GetDir) (Variables|Default|GetInterval))) (* (Math|Random|RandomFloatinRange (* -1.0 _randomrange) _randomrange) (Variables|Default|GetRandomPannerMask))) (Variables|Default|GetPanner)) _rotationpanner "1.000000,1.000000,1.000000") false)))
      (elif (== (Math|Integer|%(Integer) _index 2) 0)
        (Components|InstancedStaticMesh|AddInstance (Variables|Default|GetTile) (Math|Transform|MakeTransform (+ (+ (* _index (* (Variables|Default|GetDir) (Variables|Default|GetInterval))) (* (Math|Random|RandomFloatinRange (* -1.0 _randomrange) _randomrange) (Variables|Default|GetRandomPannerMask))) (Variables|Default|GetPanner)) _rotationpanner _scale) false)
        (else
          (Components|InstancedStaticMesh|AddInstance (Variables|Default|GetTile) (Math|Transform|MakeTransform (+ (* _index (* (Variables|Default|GetDir) (Variables|Default|GetInterval))) (* (Math|Random|RandomFloatinRange (* -1.0 _randomrange) _randomrange) (Variables|Default|GetRandomPannerMask))) "0, 0, 0" _scale) false))))))