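; BP_TilingRoof is a building art actor that procedurally lays out a grid of roof tiles.
; Its construction script loops over rows and tiles, offsetting each by a row vector and a spacing along a direction, with one shared rotation.
; Tiles alternate by column parity between two instanced mesh components, RoofTile and RoofTileSample, and InvertSort swaps which comes first.
; The event graph has no active logic.
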(event EventBeginPlay)

(event Collision|EventActorBeginOverlap
  (params (OtherActor :type Actor%20Object%20Reference)))

(event EventTick
  (params (DeltaSeconds :type Float%20%28single-precision%29)))

(fn ConstructionScript
  (bind _rotation (Variables|Default|GetRotation))
  (for _index (range 0 (- (Variables|Default|GetRowNum) 1))
    (for _index_2 (range 0 (- (Variables|Default|GetNum) 1))
      (if (Variables|Default|GetInvertSort)
        (if (== (Math|Integer|%(Integer) _index_2 2) 0)
          (Components|InstancedStaticMesh|AddInstance (Variables|Default|GetRoofTile) (Math|Transform|MakeTransform (+ (* (Variables|Default|GetRowPosPanner) _index) (* _index_2 (* (Variables|Default|GetDir) (Variables|Default|GetInterval)))) _rotation "1.000000,1.000000,1.000000") false)
          (else
            (Components|InstancedStaticMesh|AddInstance (Variables|Default|GetRoofTileSample) (Math|Transform|MakeTransform (+ (* (Variables|Default|GetRowPosPanner) _index) (* _index_2 (* (Variables|Default|GetDir) (Variables|Default|GetInterval)))) _rotation "1.000000,1.000000,1.000000") false)))
        (elif (== (Math|Integer|%(Integer) _index_2 2) 0)
          (Components|InstancedStaticMesh|AddInstance (Variables|Default|GetRoofTileSample) (Math|Transform|MakeTransform (+ (* (Variables|Default|GetRowPosPanner) _index) (* _index_2 (* (Variables|Default|GetDir) (Variables|Default|GetInterval)))) _rotation "1.000000,1.000000,1.000000") false)
          (else
            (Components|InstancedStaticMesh|AddInstance (Variables|Default|GetRoofTile) (Math|Transform|MakeTransform (+ (* (Variables|Default|GetRowPosPanner) _index) (* _index_2 (* (Variables|Default|GetDir) (Variables|Default|GetInterval)))) _rotation "1.000000,1.000000,1.000000") false)))))))