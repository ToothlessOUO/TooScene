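; BP_TilingRandom is a construction-script tool that tiles repeated mesh instances along a line for building art.
; Each loop step adds an instance to the Tile component, stepping by a direction and interval from a panner offset.
; A random offset, limited to chosen axes by a mask, jitters each position, while rotation and scale stay uniform across all instances.
; The event graph holds no logic.
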(event EventBeginPlay)

(event Collision|EventActorBeginOverlap
  (params (OtherActor :type Actor%20Object%20Reference)))

(event EventTick
  (params (DeltaSeconds :type Float%20%28single-precision%29)))

(fn ConstructionScript
  (bind _randomrange (Variables|Default|GetRandomRange))
  (for _index (range 0 (- (Variables|Default|GetNum) 1))
    (Components|InstancedStaticMesh|AddInstance (Variables|Default|GetTile) (Math|Transform|MakeTransform (+ (+ (* _index (* (Variables|Default|GetDir) (Variables|Default|GetInterval))) (* (Math|Random|RandomFloatinRange (* -1.0 _randomrange) _randomrange) (Variables|Default|GetRandomPannerMask))) (Variables|Default|GetPanner)) (Variables|Default|GetRotationPanner) (Variables|Default|Getscale)) false)))