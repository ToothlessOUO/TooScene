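; BP_Fence is a procedural fence actor that builds a straight run of pillars and handrails in the level.
; Its Construction Script adds Num handrail instances spaced by handrail length along Dir, with adjustable offset, rotation and scale.
; Pillar instances mark the start and each segment end, and the UnClosed flag omits the final one.
; Both parts use instanced meshes, and the event graph holds no logic.
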(event EventBeginPlay)

(event Collision|EventActorBeginOverlap
  (params (OtherActor :type Actor%20Object%20Reference)))

(event EventTick
  (params (DeltaSeconds :type Float%20%28single-precision%29)))

(fn ConstructionScript
  (bind _num (Variables|Default|GetNum))
  (bind _returnvalue (- _num 1))
  (if (> (Variables|Default|GetNum) 0)
    (Components|InstancedStaticMesh|AddInstance (Variables|Default|GetPillar) (Math|Transform|MakeTransform "0, 0, 0" "0, 0, 0" "1.000000,1.000000,1.000000") false)
    (for _index (range 0 _returnvalue)
      (Components|InstancedStaticMesh|AddInstance (Variables|Default|GetHandrail) (Math|Transform|MakeTransform (+ (* _index (Variables|Default|GetDir) (Variables|Default|GetHandrailLengh)) (Variables|Default|GetHandrailPanner)) (Variables|Default|GetHandrailRotation) (Variables|Default|GetHandrailScale)) false)
      (if (== _index _returnvalue)
        (if (not (Variables|Default|GetUnClosed))
          (Components|InstancedStaticMesh|AddInstance (Variables|Default|GetPillar) (Math|Transform|MakeTransform (* (+ _index 1) (Variables|Default|GetDir) (Variables|Default|GetHandrailLengh)) "0, 0, 0" "1.000000,1.000000,1.000000") false :!label _label))
        (else
          (goto _label))))))